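; BP_T1GI is a Game Instance that handles multiplayer session hosting and joining through Advanced Sessions nodes.
; CreateSession creates a session and server-travels to GameLevel as a listen server.
; JoinSession searches all server types and joins the first result, falling back to CreateSession if the search fails or finds nothing.
; A failed join only prints a debug message, as do other steps, and Init is empty.
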(event Custom|CreateSession
  (|AdvancedSession 0 (Game|GetPlayerController 0) 100 0 false true false true true true false false false true false true
    (:OnSuccess
      (Development|PrintString "Create Session!!!" true true "(R=0.155565,G=1.000000,B=0.000000,A=1.000000)" 1e+01)
      (Class|AdvancedSessionsLibrary|ServerTravel "/Game/Maps/GameLevel?listen" false false))
    (:OnFailure
      (Development|PrintString "Create Session Fail!!!" true true "(R=1.000000,G=0.102444,B=0.000000,A=1.000000)" 1e+01))))

(event Custom|JoinSession
  (bind _results (|FindSessionsAdvanced (Game|GetPlayerController 0) 0 false "AllServers" 0 false false false true)
    (:OnSuccess
      (Development|PrintString (Utilities|String|Append "Session Count : " (Utilities|String|ToString(Integer) (Utilities|Array|Length _results))) true true "(R=1.000000,G=0.000000,B=0.782032,A=1.000000)" 1e+01)
      (if (Math|Conversions|ToBoolean(Integer) (Utilities|Array|Length _results))
        (Development|PrintString "Find Session!!!" true true "(R=0.155565,G=1.000000,B=0.000000,A=1.000000)" 1e+01)
        (|JoinSession (Game|GetPlayerController 0) (Utilities|Array|Get(acopy) _results)
          (:OnSuccess
            (Development|PrintString "Join Session!!!" true true "(R=0.155565,G=1.000000,B=0.000000,A=1.000000)" 1e+01))
          (:OnFailure
            ;[1 1 1] 수정 //
            (Development|PrintString "Join Session Fail!!!" true true "(R=1.000000,G=0.104782,B=0.000000,A=1.000000)" 1e+01)))
        (else
          (Development|PrintString "22222 Find Session Fail!!!" true true "(R=1.000000,G=0.102444,B=0.000000,A=1.000000)" 1e+01)
          (CallFunction|CreateSession))))
    (:OnFailure
      (Development|PrintString "11111 Find Session Fail!!!" true true "(R=1.000000,G=0.102444,B=0.000000,A=1.000000)" 1e+01)
      (CallFunction|CreateSession))))

(event EventInit)